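; Anatomy minigame manager that asks the player to hit a randomly chosen bone on BP_Human actors until a target number of correct hits triggers the win.
; It binds to each human's bone-hit event, maps the bone name's prefix before the first underscore to a sound in ValidBones, and plays it.
; A matching hit raises the count and picks a new bone, shown as a HUD tip through BPI_PlayerHUD.
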(event Custom|OnHitBone
  (params (Bone :type Name))
  (bind (_sound _bonename) (CallFunction|CheckValidBone Bone))
  (Development|PrintString (Utilities|String|Append "Manager: " _bonename))
  (Utilities|IsValid _sound
    (:Is%20Valid
      (Audio|PlaySound2D _sound 1.0 1.0 0.0 0 0)
      (if (Utilities|Enum|Equal(Enum) _bonename (Variables|Default|GetCurrentBone))
        (if (< (Variables|Default|GetEquals) (Variables|Default|GetTargetEquals))
          (CallFunction|AddEquals))))))

(event EventBeginPlay
  (|CallParentFunction)
  (bind _outactors (Actor|GetAllActorsOfClass "/Game/VikingsPlay/GameLogic/Blueprints/MiniGames/Anatomy/BP_Human.BP_Human_C"))
  (for _array_element _outactors
    (EventDispatchers|AssignOnHitBone _array_element (delegate Custom|OnHitBone)))
  (CallFunction|GenerateQuestion))

(event EventOnPlayerWin
  (|CallParentFunction)
  (Development|PrintString "You won!"))

(fn ConstructionScript
  (|CallParentFunction))

(fn CheckValidBone
  (params (Bone :type Name))
  (bind _output_get (LocalVariables|SetBoneStrings (Utilities|String|ParseIntoArray (Utilities|String|ToString(Name) Bone) "_")))
  (if (Utilities|Array|IsValidIndex _output_get)
    (LocalVariables|SetResult (.Value (Utilities|Map|Find (Variables|Default|GetValidBones) (Utilities|Array|Get(acopy) _output_get)))))
  (return (LocalVariables|GetResult) (Utilities|Array|Get(acopy) _output_get)))

(fn AddEquals
  (Math|Integer|IncrementInt (Variables|Default|GetEquals)
    (:%20%20
      (if (== (Variables|Default|GetEquals) (Variables|Default|GetTargetEquals))
        (Default|CallOnWin)
        (else
          (CallFunction|GenerateQuestion))))))

(fn GenerateQuestion
  (bind _returnvalue (Game|GetPlayerController 0))
  (bind _returnvalue_2 (HUD|GetHUD _returnvalue))
  (bind _keys (Utilities|Map|Keys (Variables|Default|GetValidBones)))
  (Variables|Default|SetCurrentBone (.OutItem (Utilities|Array|Random _keys)))
  (Utilities|IsValid _returnvalue
    (:Is%20Valid
      (Utilities|IsValid _returnvalue_2
        (:Is%20Valid
          (if (Utilities|DoesObjectImplementInterface _returnvalue_2 "/Game/VikingsPlay/GameLogic/Blueprints/Interfaces/BPI_PlayerHUD.BPI_PlayerHUD_C")
            (Class|BPIPlayerHUD|SetTip(Message) _returnvalue_2 (Utilities|Text|ToText(String) (Variables|Default|GetCurrentBone)))))))))