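; BP_Letter is a touchable letter tile actor for the MakeWord minigame.
; Touch end (or TestTouch) broadcasts OnTouched with the tile, while SetIsSelected plays or reverses the Up timeline to lift it from its starting location.
; SetLetter takes a 1-based index, async-loads the matching texture and applies it to the cube through a new dynamic material instance.
; ResetSelected clears selection and rewinds the timeline.
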(event Custom|SetLetter
  (params (LetterIndex :type Integer))
  (bind _cube (Variables|Default|GetCube))
  (bind _textures (Variables|Default|GetTextures))
  (bind _returnvalue (Utilities|Array|Length _textures))
  (bind _returnvalue_2 (Rendering|Material|GetMaterial _cube 0))
  (if (>= _returnvalue 0)
    (if (Math|Integer|InRange(Integer) LetterIndex 1 _returnvalue)
      (bind _output_get (Variables|Default|SetLetterIndex LetterIndex))
      (bind _object (Utilities|AsyncLoadAsset (Utilities|Array|Get(acopy) (Variables|Default|GetTextures) (- _output_get 1)))
        (:Completed
          (bind _astexture_2d (Utilities|Casting|CastToTexture2D _object))
          (Utilities|IsValid _returnvalue_2
            (:Is%20Valid
              (bind _returnvalue_3 (Rendering|Material|GetBaseMaterial _returnvalue_2))
              (bind _returnvalue_4 (Rendering|Material|CreateDynamicMaterialInstance _returnvalue_3 "None" "None" :!class /Script/Engine.KismetMaterialLibrary))
              (Rendering|Material|SetTextureParameterValue _returnvalue_4 "Texture" _astexture_2d)
              (Rendering|Material|SetMaterial (Variables|Default|GetCube) 0 _returnvalue_4))))))))

(event Custom|OnTouchEnd
  (params (FingerIndex :type ETouchIndex%20Enum :default "Touch1") (TouchedActor :type Actor%20Object%20Reference))
  (Default|CallOnTouched self))

(event Custom|TestTouch
  (Default|CallOnTouched self))

(event Custom|SetIsSelected
  (params (Selected :type Boolean))
  (bind _output_get (Variables|Default|SetIsSelected Selected))
  (if _output_get
    (bind _newtrack_0 (Timeline|Up Play)
      (:Update
        (Transformation|SetActorLocation (+ (Variables|Default|GetBaseLocation) (Math|Vector|MakeVector 0.0 0.0 (* _newtrack_0 (Variables|Default|GetUpLenght)))) false true)))
    (else
      (Timeline|Up Reverse))))

(event Custom|ResetSelected
  (Variables|Default|SetIsSelected false)
  (Utilities|FlowControl|Sequence
    (:then_0
      (bind _newtrack_0 (Timeline|Up Stop)
        (:Update
          (Transformation|SetActorLocation (+ (Variables|Default|GetBaseLocation) (Math|Vector|MakeVector 0.0 0.0 (* _newtrack_0 (Variables|Default|GetUpLenght)))) false true))))
    (:then_1
      (Timeline|Up SetNewTime))))

(event EventBeginPlay
  (EventDispatchers|AssignOnInputTouchEnd (delegate Custom|OnTouchEnd))
  (Variables|Default|SetBaseLocation (Transformation|GetActorLocation)))

(fn ConstructionScript)

(fn GetLetterIndex
  (return (Variables|Default|GetLetterIndex)))

(fn GetIsSelected
  (return (Variables|Default|GetIsSelected)))