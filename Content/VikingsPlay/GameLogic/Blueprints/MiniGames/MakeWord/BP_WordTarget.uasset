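; BP_WordTarget is a target actor for the MakeWord minigame that shows a random mesh paired with a word.
; On BeginPlay it picks a random key from the Targets map, async loads that mesh and applies it to its StaticMesh component.
; The matching value's Indexes become CurrentWord, set without waiting for the load and exposed through GetCurrentWord.
; The actor destroys itself if Targets is empty.
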(event EventBeginPlay
  (if (> (Utilities|Map|Length (Variables|Default|GetTargets)) 0)
    (bind _keys (Utilities|Map|Keys (Variables|Default|GetTargets)))
    (bind _output_get (Variables|Default|SetCurrentIndex (.OutIndex (Utilities|Array|Random _keys))))
    (bind _object (Utilities|AsyncLoadAsset (Utilities|Array|Get(acopy) _keys _output_get))
      (:then
        (bind _values (Utilities|Map|Values (Variables|Default|GetTargets)))
        (Variables|Default|SetCurrentWord (.indexes (Utilities|Array|Get(acopy) _values (Variables|Default|GetCurrentIndex)))))
      (:Completed
        (bind _asstatic_mesh (Utilities|Casting|CastToStaticMesh _object))
        (Components|StaticMesh|SetStaticMesh (Variables|Default|GetStaticMesh) _asstatic_mesh)))
    (else
      (Actor|DestroyActor))))

(fn ConstructionScript)

(fn GetCurrentWord
  (return (Variables|Default|GetCurrentWord)))