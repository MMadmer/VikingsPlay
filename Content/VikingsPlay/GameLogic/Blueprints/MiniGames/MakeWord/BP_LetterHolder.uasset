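; Letter slot for the MakeWord minigame that holds one letter and knows which letter belongs in it.
; On BeginPlay it binds touch-end input, which broadcasts OnTouched with itself, as does the TestTouch event.
; SetCurrentLetter stores the given letter and broadcasts OnPutRightLetter when that letter is valid and its index matches TargetLetter.
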(event Custom|OnTouchEnd
  (params (FingerIndex :type ETouchIndex%20Enum :default "Touch1") (TouchedActor :type Actor%20Object%20Reference))
  (Default|CallOnTouched self))

(event Custom|TestTouch
  (Default|CallOnTouched self))

(event EventBeginPlay
  (EventDispatchers|AssignOnInputTouchEnd (delegate Custom|OnTouchEnd)))

(fn ConstructionScript)

(fn SetCurrentLetter
  (params (Letter :type BP%20Letter%20Object%20Reference))
  (bind _output_get (Variables|Default|SetCurrentLetter Letter))
  (Utilities|IsValid _output_get
    (:Is%20Valid
      (if (== (Default|GetLetterIndex (Variables|Default|GetCurrentLetter)) (Variables|Default|GetTargetLetter))
        (Default|CallOnPutRightLetter self)))))

(fn GetCurrentLetter
  (return (Variables|Default|GetCurrentLetter)))