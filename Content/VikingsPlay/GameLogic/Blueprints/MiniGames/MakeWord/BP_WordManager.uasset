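; Manager for the MakeWord minigame, where the player touches letters and holders to assemble a target word.
; Once the UTPrefab loads, it reads BP_WordTarget, clones a row of holders from the first one, and hides the word among randomized letters.
; A selected letter snaps into a touched holder; touching a filled one returns it to the prefab component matching its name.
; Correct placements trigger a full-word check that fires OnWin.
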(event Custom|OnOwningPrefabLoaded
  (CallFunction|StartGame))

(event Custom|StartGame
  (bind _holders (Variables|Main|GetHolders))
  (bind _output (Utilities|Array|Get(acopy) _holders))
  (bind _returnvalue (Transformation|GetActorTransform _output))
  (bind _word (CallFunction|TryFindCurrentWord))
  (Variables|Main|SetCurrentWord _word)
  (bind _letters (CallFunction|TryFindLetters))
  (Variables|Main|SetLetters _letters)
  (bind _holder (CallFunction|TryFindLetterHolder))
  (Utilities|Array|Add (Variables|Main|GetHolders) _holder)
  (if (CallFunction|CanStartGame)
    (for (_array_element _array_index) (Variables|Main|GetCurrentWord)
      (CallFunction|SetRandomLetter _array_element)
      (if (== _array_index 0)
        _
        (else
          (bind _returnvalue_2 (Game|SpawnActorfromClass "/Game/VikingsPlay/GameLogic/Blueprints/MiniGames/MakeWord/BP_LetterHolder.BP_LetterHolder_C" (Math|Transform|MakeTransform (+ (.location _returnvalue) (* (Math|Vector|NegateVector (Transformation|GetActorRightVector _output)) (* _array_index (+ (* (.y (.BoxExtent (Collision|GetActorBounds _output false false))) 2.0) 5.0)))) (.rotation _returnvalue) (.scale _returnvalue)) "AlwaysSpawn" (Variables|Main|GetOwningPrefab) 0))
          (Utilities|Array|Add (Variables|Main|GetHolders) _returnvalue_2)))
      (Variables|/Game/VikingsPlay/GameLogic/Blueprints/MiniGames/MakeWord/BP_LetterHolder.BP_LetterHolder_C|SetTargetLetter (Utilities|Array|Get(acopy) (Variables|Main|GetHolders) _array_index) _array_element))
    (for _array_element_2 (Variables|Main|GetHolders)
      (EventDispatchers|AssignOnTouched _array_element_2 (delegate Custom|OnHolderTouched))
      (EventDispatchers|AssignOnPutRightLetter _array_element_2 (delegate Custom|OnPutRightLetter)))
    (for (_array_element_3 _array_index_2) (Variables|Main|GetLetters)
      (EventDispatchers|AssignOnTouched _array_element_3 (delegate Custom|OnLetterTouched))
      (if (not (Utilities|Set|Contains (Variables|Default|GetUsedLetters) _array_index_2))
        (Default|SetLetter _array_element_3 (Math|Random|RandomIntegerinRange 1 33))))
    (else
      (Actor|DestroyActor))))

(event Custom|OnHolderTouched
  (params (Holder :type BP%20Letter%20Holder%20Object%20Reference))
  (Utilities|IsValid (Default|GetCurrentLetter Holder)
    (:Is%20Valid
      (CallFunction|ClearHolder Holder))
    (:Is%20Not%20Valid
      (Utilities|IsValid (Variables|Default|GetLastSelectedLetter)
        (:Is%20Valid
          (if (Default|GetIsSelected (Variables|Default|GetLastSelectedLetter))
            (Default|ResetSelected (Variables|Default|GetLastSelectedLetter))
            (Transformation|AttachComponentToComponent (Variables|Default|GetLastSelectedLetter) (Variables|/Game/VikingsPlay/GameLogic/Blueprints/MiniGames/MakeWord/BP_LetterHolder.BP_LetterHolder_C|GetLetterPlace Holder) "None" "SnapToTarget" "SnapToTarget" "SnapToTarget" true)
            (Default|SetCurrentLetter Holder (Variables|Default|GetLastSelectedLetter))
            (else
              (Variables|Default|SetLastSelectedLetter 0))))))))

(event Custom|OnLetterTouched
  (params (Letter :type BP%20Letter%20Object%20Reference))
  (bind _holder (CallFunction|IsLetterinHolder Letter))
  (Utilities|IsValid _holder
    (:Is%20Valid
      (CallFunction|ClearHolder _holder))
    (:Is%20Not%20Valid
      (Default|SetIsSelected Letter (not (Default|GetIsSelected Letter)))
      (if (!= (Variables|Default|GetLastSelectedLetter) Letter)
        (if (Default|GetIsSelected Letter)
          (Variables|Default|SetLastSelectedLetter Letter)
          (else
            (Variables|Default|SetLastSelectedLetter 0)))))))

(event Custom|OnPutRightLetter
  (params (Holder :type BP%20Letter%20Holder%20Object%20Reference))
  (bind _result (CallFunction|CheckWin))
  (if _result
    (Default|CallOnWin)))

(event EventBeginPlay
  (bind _outactors (Actor|GetAllActorsOfClass "/Script/UsefulTools.UTPrefab"))
  (if (Utilities|Array|IsValidIndex _outactors)
    (bind _output_get (Variables|Main|SetOwningPrefab (Utilities|Array|Get(acopy) _outactors)))
    (Utilities|IsValid _output_get
      (:Is%20Valid
        (if (Class|UTPrefab|IsPrefabLoaded (Variables|Main|GetOwningPrefab))
          (CallFunction|StartGame)
          (else
            (EventDispatchers|AssignOnPrefabLoaded (Variables|Main|GetOwningPrefab) (delegate Custom|OnOwningPrefabLoaded))))))))

(fn ConstructionScript)

(fn TryFindOwningPrefab
  (bind _outactors (Actor|GetAllActorsOfClass "/Script/UsefulTools.UTPrefab"))
  (if (Utilities|Array|IsValidIndex _outactors)
    (LocalVariables|SetFoundPrefab (Utilities|Array|Get(acopy) _outactors)))
  (return (LocalVariables|GetFoundPrefab)))

(fn TryFindCurrentWord
  (bind _outactors (Actor|GetAllActorsOfClass "/Game/VikingsPlay/GameLogic/Blueprints/MiniGames/MakeWord/BP_WordTarget.BP_WordTarget_C"))
  (if (Utilities|Array|IsValidIndex _outactors)
    (bind _word (Default|GetCurrentWord (Utilities|Array|Get(acopy) _outactors)))
    (LocalVariables|SetFoundWord _word))
  (return (LocalVariables|GetFoundWord)))

(fn TryFindLetters
  (bind _outactors (Actor|GetAllActorsOfClass "/Game/VikingsPlay/GameLogic/Blueprints/MiniGames/MakeWord/BP_Letter.BP_Letter_C"))
  (bind _output_get (LocalVariables|SetFoundLetters _outactors))
  (return _output_get))

(fn TryFindLetterHolder
  (bind _outactors (Actor|GetAllActorsOfClass "/Game/VikingsPlay/GameLogic/Blueprints/MiniGames/MakeWord/BP_LetterHolder.BP_LetterHolder_C"))
  (if (Utilities|Array|IsValidIndex _outactors)
    (LocalVariables|SetFoundHolder (Utilities|Array|Get(acopy) _outactors)))
  (return (LocalVariables|GetFoundHolder)))

(fn CanStartGame
  (bind _currentword (Variables|Main|GetCurrentWord))
  (bind _letters (Variables|Main|GetLetters))
  (bind _returnvalue (Utilities|Array|Length _currentword))
  (bind _returnvalue_2 (Utilities|Array|Length _letters))
  (if (Math|Boolean|ANDBoolean (> _returnvalue 0) (> _returnvalue_2 0) (>= _returnvalue_2 _returnvalue) (Utilities|Array|IsValidIndex (Variables|Main|GetHolders)))
    (Utilities|IsValid (Utilities|Array|Get(acopy) (Variables|Main|GetHolders))
      (:Is%20Valid
        (LocalVariables|SetCan true))
      (:Is%20Not%20Valid
        _)))
  (return (LocalVariables|GetCan)))

(fn SetRandomLetter
  (params (Letter :type Integer))
  (bind _output_get (LocalVariables|SetIndex (.OutIndex (Utilities|Array|Random (Variables|Main|GetLetters)))))
  (while (Utilities|Set|Contains (Variables|Default|GetUsedLetters) _output_get)
    (LocalVariables|SetIndex (Math|Integer|%(Integer) (+ (LocalVariables|GetIndex) 1) (Utilities|Array|Length (Variables|Main|GetLetters)))))
  (Default|SetLetter (Utilities|Array|Get(acopy) (Variables|Main|GetLetters) (LocalVariables|GetIndex)) Letter)
  (Utilities|Set|Add (Variables|Default|GetUsedLetters) (LocalVariables|GetIndex)))

(fn ClearHolder
  (params (Holder :type BP%20Letter%20Holder%20Object%20Reference))
  (bind _currentletter (Default|GetCurrentLetter Holder))
  (Utilities|IsValid Holder
    (:Is%20Valid
      (Utilities|IsValid (Default|GetCurrentLetter Holder)
        (:Is%20Valid
          (Utilities|IsValid (Variables|Main|GetOwningPrefab)
            (:Is%20Valid
              (bind _output_get (LocalVariables|SetSceneComponents (Actor|GetComponentsByClass (Variables|Main|GetOwningPrefab) "/Script/Engine.SceneComponent")))
              (bind _array_element (Utilities|Array|ForEachLoopwithBreak _output_get :!label _label)
                (:LoopBody
                  (if (Utilities|Enum|Equal(Enum) (Utilities|GetObjectName _array_element) (Utilities|GetObjectName (Default|GetCurrentLetter Holder)))
                    (LocalVariables|SetValidSceneComp _array_element)
                    (goto _label Break)))
                (:Completed
                  (Utilities|IsValid (LocalVariables|GetValidSceneComp)
                    (:Is%20Valid
                      (Transformation|AttachComponentToComponent _currentletter (LocalVariables|GetValidSceneComp) "None" "SnapToTarget" "SnapToTarget" "SnapToTarget" true)
                      (Default|ResetSelected _currentletter)
                      (Default|SetCurrentLetter Holder))))))))))))

(fn IsLetterinHolder
  (params (Letter :type BP%20Letter%20Object%20Reference))
  (bind _array_element (Utilities|Array|ForEachLoopwithBreak (Variables|Main|GetHolders) :!label _label)
    (:LoopBody
      (if (== Letter (Default|GetCurrentLetter _array_element))
        (LocalVariables|SetResult true)
        (LocalVariables|SetFoundHolder _array_element)
        (goto _label Break)))
    (:Completed
      (return (LocalVariables|GetResult) (LocalVariables|GetFoundHolder)))))

(fn CheckWin
  (if (== (Utilities|Array|Length (Variables|Main|GetHolders)) (Utilities|Array|Length (Variables|Main|GetCurrentWord)))
    (for (_array_element _array_index) (Variables|Main|GetHolders)
      (Utilities|IsValid (Default|GetCurrentLetter _array_element)
        (:Is%20Valid
          (if (== (Default|GetLetterIndex (Default|GetCurrentLetter _array_element)) (Utilities|Array|Get(acopy) (Variables|Main|GetCurrentWord) _array_index))
            (Math|Integer|IncrementInt (LocalVariables|GetEquals))))))
    (return (== (LocalVariables|GetEquals) (Utilities|Array|Length (Variables|Main|GetCurrentWord))))))