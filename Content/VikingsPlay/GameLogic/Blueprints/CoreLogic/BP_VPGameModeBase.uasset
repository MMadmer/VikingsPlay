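; BP_VPGameModeBase is a game mode that runs an AR session and places prefabs on planes the player touches.
; On BeginPlay it starts AR, disables the screensaver, registers the touch callback with VPARSubsystem and loads the current prefab.
; LoadPrefab sets the prefab class, destroys existing UTPrefab actors and enables scanning.
; A plane touch stops scanning and spawns the prefab at that plane's transform, if the class is valid.
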(event Custom|OnPlayerTouchedPlane
  (params (PlaneGeometry :type AR%20Plane%20Geometry%20Object%20Reference) (PlayerController :type Player%20Controller%20Object%20Reference))
  (if (Utilities|IsValidClass (Variables|Default|GetCurrentPrefab))
    (Class|VPARSubsystem|SetIsScanActive (Subsystems|GetVPARSubsystem) false)
    (Game|SpawnActorfromClass (Variables|Default|GetCurrentPrefab) (Class|ARTrackedGeometry|GetLocaltoWorldTransform PlaneGeometry) "AlwaysSpawn" 0 0)
    (else
      (Development|PrintString "Not valid prefab class" true true "(R=1.000000,G=0.703681,B=0.000000,A=1.000000)" 1e+01))))

(event EventBeginPlay
  (Class|ARBlueprintLibrary|StartARSession "/Game/VikingsPlay/GameLogic/D_ARSessionConfig.D_ARSessionConfig")
  (Class|KismetSystemLibrary|ControlScreensaver false)
  (EventDispatchers|AssignOnPlayerTouchedPlane (Subsystems|GetVPARSubsystem) (delegate Custom|OnPlayerTouchedPlane))
  (CallFunction|LoadPrefab (Variables|Default|GetCurrentPrefab)))

(event EventLoadPrefab
  (params (Prefab :type BP%20Prefab%20Base%20Class%20Reference))
  (Variables|Default|SetCurrentPrefab Prefab)
  (bind _outactors (Actor|GetAllActorsOfClass "/Script/UsefulTools.UTPrefab"))
  (for _array_element _outactors
    (Actor|DestroyActor _array_element))
  (Class|VPARSubsystem|SetIsScanActive (Subsystems|GetVPARSubsystem) true)
  (Development|PrintString (Utilities|GetClassDisplayName (Variables|Default|GetCurrentPrefab)) true true "(R=0.000000,G=0.660000,B=1.000000,A=1.000000)" 1e+01))

(fn ConstructionScript)