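; BP_Widget is a touchable level object that asks the game mode to load a target prefab.
; A touch release on the actor, or the TestTouch event, passes through a DoOnce with no reset and plays a timeline that animates the actor's scale.
; When the animation finishes, it sends LoadPrefabMessage with TargetPrefab to the game mode, provided that implements BPI_MiniGames.
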(event Custom|OnTouchEnd
  (params (FingerIndex :type ETouchIndex%20Enum :default "Touch1") (TouchedActor :type Actor%20Object%20Reference))
  (bind _returnvalue (Game|GetGameMode))
  (Utilities|FlowControl|DoOnce false
    (:Completed
      (bind _newtrack_0 (Timeline|Animation PlayFromStart)
        (:Update
          (Transformation|SetActorScale3D (Math|Conversions|ToVector(Float) _newtrack_0)))
        (:Finished
          (if (Utilities|DoesObjectImplementInterface _returnvalue "/Game/VikingsPlay/GameLogic/Blueprints/Interfaces/BPI_MiniGames.BPI_MiniGames_C")
            (Class|BPIMiniGames|LoadPrefab(Message) _returnvalue (Variables|Default|GetTargetPrefab))))))))

(event Custom|TestTouch
  (bind _returnvalue (Game|GetGameMode))
  (Utilities|FlowControl|DoOnce false
    (:Completed
      (bind _newtrack_0 (Timeline|Animation PlayFromStart)
        (:Update
          (Transformation|SetActorScale3D (Math|Conversions|ToVector(Float) _newtrack_0)))
        (:Finished
          (if (Utilities|DoesObjectImplementInterface _returnvalue "/Game/VikingsPlay/GameLogic/Blueprints/Interfaces/BPI_MiniGames.BPI_MiniGames_C")
            (Class|BPIMiniGames|LoadPrefab(Message) _returnvalue (Variables|Default|GetTargetPrefab))))))))

(event EventBeginPlay
  (EventDispatchers|AssignOnInputTouchEnd (delegate Custom|OnTouchEnd)))

(fn ConstructionScript)